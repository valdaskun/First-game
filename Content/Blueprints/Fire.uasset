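; Fire hazard for a side-scroller that damages a SideScrollerCharacter over time while it stands inside the Box trigger.
; Entering sets an in-radius flag and starts a delay loop that lowers clamped Health each second until the character leaves.
; At zero Health it calls Death on player 0's character and shows the LevelFailed widget after a short delay.
; The Damage call is disconnected, so Health is edited directly.
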(event OnComponentBeginOverlap(Box)
  (params (OverlappedComponent :type Primitive%20Component%20Object%20Reference) (OtherActor :type Actor%20Object%20Reference) (OtherComp :type Primitive%20Component%20Object%20Reference) (OtherBodyIndex :type Integer) (bFromSweep :type Boolean) (SweepResult :type Hit%20Result%20Structure%20%28by%20ref%29))
  (bind _asside_scroller_character (Utilities|Casting|CastToSideScrollerCharacter OtherActor))
  (Variables|Default|SetPlayerInRadius true)
  (bind _output_get (Variables|/Game/SideScrollerBP/Blueprints/SideScrollerCharacter.SideScrollerCharacter_C|SetHealth _asside_scroller_character (Math|Float|Clamp(Float) (- (Variables|/Game/SideScrollerBP/Blueprints/SideScrollerCharacter.SideScrollerCharacter_C|GetHealth _asside_scroller_character) 0.101)) :!label _label))
  (bind _asside_scroller_character_2 (Utilities|Casting|CastToSideScrollerCharacter (Game|GetPlayerCharacter 0)))
  (if (<= _output_get 0.0)
    (Development|PrintString "why???")
    (bind _asside_scroller_character_3 (Utilities|Casting|CastToSideScrollerCharacter (Game|GetPlayerCharacter 0)))
    (Default|Death _asside_scroller_character_3)
    (bind _returnvalue (UserInterface|CreateWidget "/Game/SideScrollerBP/Blueprints/LevelFailed.LevelFailed_C"))
    (Utilities|FlowControl|Delay 2.5)
    (UserInterface|Viewport|AddtoViewport _returnvalue 0)
    (else
      (Utilities|FlowControl|Delay 1.0)
      (if (Variables|Default|GetPlayerInRadius)
        (goto _label)))))

(event OnComponentEndOverlap(Box)
  (params (OverlappedComponent :type Primitive%20Component%20Object%20Reference) (OtherActor :type Actor%20Object%20Reference) (OtherComp :type Primitive%20Component%20Object%20Reference) (OtherBodyIndex :type Integer))
  (Utilities|Casting|CastToSideScrollerCharacter OtherActor)
  (Variables|Default|SetPlayerInRadius false))

(event EventBeginPlay)

(fn ConstructionScript)