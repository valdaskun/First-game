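; Explosions is a recurring explosion hazard actor that damages the side-scroller player while they stand inside its Box.
; Box overlap events track the player's presence and print debug messages.
; From BeginPlay, a looping Delay spawns an enlarged explosion emitter and subtracts clamped Health if the player is inside.
; When Health runs out, it calls the character's Death, shows the LevelFailed widget and stops looping.
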(event OnComponentBeginOverlap(Box)
  (params (OverlappedComponent :type Primitive%20Component%20Object%20Reference) (OtherActor :type Actor%20Object%20Reference) (OtherComp :type Primitive%20Component%20Object%20Reference) (OtherBodyIndex :type Integer) (bFromSweep :type Boolean) (SweepResult :type Hit%20Result%20Structure%20%28by%20ref%29))
  (Utilities|Casting|CastToSideScrollerCharacter OtherActor)
  (Variables|Default|SetPlayerInRadius true)
  (Development|PrintString "in"))

(event OnComponentEndOverlap(Box)
  (params (OverlappedComponent :type Primitive%20Component%20Object%20Reference) (OtherActor :type Actor%20Object%20Reference) (OtherComp :type Primitive%20Component%20Object%20Reference) (OtherBodyIndex :type Integer))
  (Utilities|Casting|CastToSideScrollerCharacter OtherActor)
  (Variables|Default|SetPlayerInRadius false)
  (Development|PrintString "out"))

(event EventBeginPlay
  (bind _returnvalue (Game|GetPlayerCharacter 0))
  (bind _returnvalue_2 (Effects|SpawnEmitteratLocation "/Game/StarterContent/Particles/P_Explosion.P_Explosion" (Transformation|GetActorLocation) :!label _label))
  (Transformation|SetWorldScale3D _returnvalue_2 "3.000000,3.000000,3.000000")
  (if (Variables|Default|GetPlayerInRadius)
    (bind _asside_scroller_character (Utilities|Casting|CastToSideScrollerCharacter (Game|GetPlayerCharacter 0)))
    (bind _output_get (Variables|/Game/SideScrollerBP/Blueprints/SideScrollerCharacter.SideScrollerCharacter_C|SetHealth _asside_scroller_character (Math|Float|Clamp(Float) (- (Variables|/Game/SideScrollerBP/Blueprints/SideScrollerCharacter.SideScrollerCharacter_C|GetHealth _asside_scroller_character) 0.5))))
    (if (<= _output_get 0.0)
      (bind _asside_scroller_character_2 (Utilities|Casting|CastToSideScrollerCharacter _returnvalue))
      (Default|Death _asside_scroller_character_2)
      (bind _asside_scroller_character_3 (Utilities|Casting|CastToSideScrollerCharacter _returnvalue))
      (bind _returnvalue_3 (UserInterface|CreateWidget "/Game/SideScrollerBP/Blueprints/LevelFailed.LevelFailed_C"))
      (Default|Death _asside_scroller_character_3)
      (UserInterface|Viewport|AddtoViewport _returnvalue_3 0)
      (else
        (Utilities|FlowControl|Delay 2.0)
        (goto _label)))
    (else
      (Utilities|FlowControl|Delay 2.0)
      (goto _label))))

(fn ConstructionScript)